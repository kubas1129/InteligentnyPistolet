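; Blueprint function library of shared static helpers for the game.
; It returns the player pawn cast to BP_IntelligentViewPawn and the first BP_HeadQuarter actor found in the level.
; It also generates a random point on a hardcoded road grid, picking one of three fixed lines along a random axis and a random position along it.
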(fn `GetPawn`
  (returns (pawn :type "/Game/Blueprints/BP_IntelligentViewPawn Object Reference"))
  (return (cast `/Game/Blueprints/BP_IntelligentViewPawn` (`GameplayStatics.GetPlayerPawn` (`local.__WorldContext`)) :!pure true)))

(fn `GetQuarter`
  (returns (quarter :type "/Game/Blueprints/Model/BP_HeadQuarter Object Reference"))
  (bind _outactors (`GameplayStatics.GetAllActorsOfClass` (`local.__WorldContext`) "/Game/Blueprints/Model/BP_HeadQuarter.BP_HeadQuarter_C"))
  (if (`KismetArrayLibrary.Array_IsValidIndex` _outactors)
    (return (`|GetArrayItem` _outactors))))

(fn `GetRandomPointOnRoad`
  (returns (point :type "Vector Structure"))
  (if (`KismetMathLibrary.RandomBool`)
    (return (`KismetMathLibrary.MakeVector` (select `int` (`KismetMathLibrary.RandomIntegerInRange` 0 2) :`0` -1900.0 :`1` -1000.0 :`2` -300.0 :!type "Float (single-precision)") (`KismetMathLibrary.RandomFloatInRange` -1450.0 1450.0) 20.0))
    (else
      (return (`KismetMathLibrary.MakeVector` (`KismetMathLibrary.RandomFloatInRange` -2500.0 450.0) (select `int` (`KismetMathLibrary.RandomIntegerInRange` 0 2) :`0` -1100.0 :`1` -100.0 :`2` 500.0 :!type "Float (single-precision)") 20.0)))))