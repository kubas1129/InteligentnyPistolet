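; Threat manager that randomly spawns threat events at road locations during play, up to a maximum count.
; BeginPlay caches all BP_PlaceToSpawn actors as roads.
; Each Tick requires two weighted random rolls on the same chance to pass, squaring the effective probability, before spawning.
; Each BP_ThreatEvent gets a random ID, Normal or High priority and the HeadQuarter reference, then is tracked and logged.
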(event `self.ReceiveBeginPlay`
  ;[1 1 1] Set roads array
  (bind _outactors (`GameplayStatics.GetAllActorsOfClass` "/Game/Blueprints/Threats/BP_PlaceToSpawn.BP_PlaceToSpawn_C"))
  (set `self.roads` _outactors))

(event `self.ReceiveTick`
  (params (DeltaSeconds :type "Float (single-precision)"))
  (if (and (and (`KismetMathLibrary.RandomBoolWithWeight` (`self.chanceToAddThreat`)) (`KismetMathLibrary.RandomBoolWithWeight` (`self.chanceToAddThreat`))) (< (`KismetArrayLibrary.Array_Length` (`self.threats`)) (`self.maxThreats`)))
    (`self.RandomSpawnThreat`)))

(fn `RandomSpawnThreat`
  (bind _returnvalue (`|SpawnActorFromClass` "/Game/Blueprints/Threats/BP_ThreatEvent.BP_ThreatEvent_C" (`KismetMathLibrary.MakeTransform` (`/Game/Blueprints/All/StaticLib.GetRandomPointOnRoad`)) "Undefined" "OverrideRootScale" self (make `ThreatInfo` (`KismetMathLibrary.RandomIntegerInRange` 1 99999) (select `int` (`KismetMathLibrary.RandomIntegerInRange` 0 1) :`0` "OP_Normal" :`1` "OP_High" :!type "EOrderPriority Enum")) (`self.headQuarter`) null))
  (`KismetArrayLibrary.Array_Add` (`self.threats`) _returnvalue)
  (bind (_threatid _orderpriority) (break `ThreatInfo` (`/Game/Blueprints/Threats/BP_ThreatEvent.threatInfo` _returnvalue)))
  (`CBlueprintFunctionLibrary.AddToLog` (`KismetStringLibrary.Concat_StrStr` " Threat " (`KismetStringLibrary.Conv_IntToString` _threatid) " was created with priority " (`|GetEnumeratorNameAsString` _orderpriority))))

(fn `UserConstructionScript`)