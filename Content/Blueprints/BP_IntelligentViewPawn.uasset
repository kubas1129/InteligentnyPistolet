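; Player view pawn for a map of patrols, headquarters, policemen, ambulances and threat events, handling navigation, selection and the HUD.
; Scroll input moves the pawn's height within limits, and holding the move input pans it by mouse delta scaled by that height.
; Selecting an actor updates its outline, clears goal markers and rebuilds an info widget for recognized actor types.
; Follow events only store or clear the target actor reference.
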(event `self.ReceiveBeginPlay`
  (bind (_returnvalue_x _returnvalue_y _returnvalue_z) (`KismetMathLibrary.BreakVector` (`self.K2_GetActorLocation`)))
  (set `self.defaultScroll` _returnvalue_z)
  (bind _returnvalue (`|CreateWidget` "/Game/Widgets/WB_HUD.WB_HUD_C" (`GameplayStatics.GetPlayerController` 0)))
  (`UserWidget.AddToViewport` _returnvalue 0))

(event `/Game/Blueprints/All/BP_FollowInterface.StartFollowActor`
  (params (actorRef :type "Actor Object Reference"))
  (set `self.followActor` actorRef))

(event `/Game/Blueprints/All/BP_FollowInterface.StopFollowActor`
  (set `self.followActor` null))

(event `InputAction|ScrollUp`
  (params (Key :type "Key Structure"))
  ;[1 1 1] Scroll
  (:`Pressed`
    (`self.ScrollAction` true)))

(event `InputAction|ScrollDown`
  (params (Key :type "Key Structure"))
  ;[1 1 1] Scroll
  (:`Pressed`
    (`self.ScrollAction` false)))

(event `InputAxis|MoveModeActivate`
  (params (AxisValue :type "Float (single-precision)"))
  (bind (_lastmouseposition_x _lastmouseposition_y) (`KismetMathLibrary.BreakVector2D` (`self.lastMousePosition`)))
  (bind (_locationx _locationy) (`WidgetLayoutLibrary.GetMousePositionScaledByDPI` (`GameplayStatics.GetPlayerController` 0)))
  (bind _returnvalue (`KismetMathLibrary.MakeVector2D` _locationx _locationy))
  (bind _returnvalue_2 (`KismetMathLibrary.Lerp` 2.0 1.0 (/ (`self.scrollCurrent`) (`self.scrollMax`))))
  (bind (_x _y) (`KismetMathLibrary.BreakVector2D` _returnvalue))
  ;[1 1 1] Move screen on map
  (`/Engine/EditorBlueprintResources/StandardMacros.CompareFloat` AxisValue 1.0
    (:`==`
      (`self.K2_AddActorWorldOffset` (`KismetMathLibrary.MakeVector` (/ (* (- _lastmouseposition_y _y) -1.0) _returnvalue_2) (/ (- _lastmouseposition_x _x) _returnvalue_2)))
      (set `self.lastMousePosition` _returnvalue))
    (:`<`
      (set `self.lastMousePosition` _returnvalue))))

(event `SetCurrentClickActor`
  (params (currentClickedActor :type "Actor Object Reference"))
  (bind _currentclickedactor (`self.currentClickedActor`))
  ;[1 1 1] Set new clicked actor
  (`/Engine/EditorBlueprintResources/StandardMacros.IsValid` _currentclickedactor
    (:`Is Valid`
      (message `/Game/Blueprints/All/BP_OutlineInterface.DisableOutline` _currentclickedactor))
    (:`Is Not Valid`
      _))
  (`/Engine/EditorBlueprintResources/StandardMacros.IsValid` currentClickedActor
    (:`Is Valid`
      (bind _output_get (set `self.currentClickedActor` currentClickedActor))
      (message `/Game/Blueprints/All/BP_OutlineInterface.EnableOutline` _output_get)
      (`self.ChangeInfoWidget`)
      (bind _outactors (`GameplayStatics.GetAllActorsOfClass` "/Game/Blueprints/Threats/BP_GoalRepresentation.BP_GoalRepresentation_C"))
      (for _array_element _outactors
        (`self.K2_DestroyActor` _array_element)))))

(event `ChangeInfoWidget`
  (bind _currentwidgetinfo (`self.currentWidgetInfo`))
  (bind _currentclickedactor (`self.currentClickedActor`))
  (bind _type (`self.GetActorTypeFromClass` (`GameplayStatics.GetObjectClass` _currentclickedactor)))
  ;[1 1 1] Widget info
  (`/Engine/EditorBlueprintResources/StandardMacros.IsValid` _currentwidgetinfo
    (:`Is Valid`
      (`Widget.RemoveFromParent` _currentwidgetinfo))
    (:`Is Not Valid`
      _))
  (if (`|EnumInequality` _type "NewEnumerator6")
    (bind _returnvalue (`|CreateWidget` "/Game/Widgets/WB_SelectedActorInfo.WB_SelectedActorInfo_C" (`GameplayStatics.GetPlayerController` 0) _currentclickedactor _type))
    (bind _output_get (set `self.currentWidgetInfo` _returnvalue))
    (`UserWidget.AddToViewport` _output_get 0)))

(fn `GetActorTypeFromClass`
  (params (class :type "Actor Class Reference"))
  (returns (type :type "/Game/Blueprints/All/EActorSelectedType Enum"))
  (castclass `CPatrol` class
    (:`then`
      (return "NewEnumerator0"))
    (:`CastFailed`
      (castclass `CHeadQuarter` class
        (:`then`
          (return "NewEnumerator2"))
        (:`CastFailed`
          (castclass `CPoliceman` class
            (:`then`
              (return "NewEnumerator1"))
            (:`CastFailed`
              (castclass `CAmbulance` class
                (:`then`
                  (return "NewEnumerator3"))
                (:`CastFailed`
                  (castclass `/Game/Blueprints/Threats/BP_ThreatEvent` class
                    (:`then`
                      (return "NewEnumerator5"))
                    (:`CastFailed`
                      (return "NewEnumerator6"))))))))))))

(fn `isActorClicked`
  (params (actor :type "Actor Object Reference"))
  (returns (actorClicked :type Boolean))
  (return (== actor (`self.currentClickedActor`))))

(fn `ScrollAction`
  (params (scrollIn :type Boolean))
  (bind (_returnvalue_x _returnvalue_y) (`KismetMathLibrary.BreakVector` (`self.K2_GetActorLocation`)))
  (set `self.scrollCurrent` (`KismetMathLibrary.FClamp` (+ (select `bool` scrollIn :`false` 100.0 :`true` -100.0 :!type "Float (single-precision)") (`self.scrollCurrent`)) (`self.scrollMin`) (`self.scrollMax`)))
  (`self.K2_SetActorLocation` (`KismetMathLibrary.MakeVector` _returnvalue_x _returnvalue_y (+ (`self.scrollCurrent`) (`self.defaultScroll`)))))

(fn `UserConstructionScript`)