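; BP_Patrol is a police patrol pawn that roams random road points and responds to crime threats.
; On spawn it attaches a navigation actor and officers; crime requests set the threat and notify each officer's smartwatch.
; A re-entrant PatrolState machine drives AI movement, destroys threats after a random delay, then asks headquarters for new orders or resumes roaming.
; Cursor hover toggles a custom-depth outline, and clicking selects the patrol and shows its goal marker.
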(event `self.ReceiveBeginPlay`
  (`self.InitSetup`)
  (`self.ActionCenter`))

(event `OnCrimeRequest`
  (params (threatRef :type "/Game/Blueprints/Threats/BP_ThreatEvent Object Reference") (orderRequest :type "SmartWatchOrderRequest Structure"))
  ;[1 1 1] On crime request
  (set `self.currentThreat` threatRef)
  (set `self.patrolState` "NewEnumerator7")
  (`self.ActionCenter`)
  (for _array_element (`self.GetOfficers`)
    (`CSmartWatch.OnOrderRequest` (`CPoliceman.GetSmartWatch` _array_element) orderRequest)))

(event `self.EnableOutline`
  ;[1 1 1] Outline interface
  (`PrimitiveComponent.SetRenderCustomDepth` (`self.Cylinder`) true))

(event `self.DisableOutline`
  ;[1 1 1] Outline interface
  (`PrimitiveComponent.SetRenderCustomDepth` (`self.Cylinder`) false))

(event `self.Cylinder.OnBeginCursorOver`
  (params (TouchedComponent :type "PrimitiveComponent Object Reference"))
  ;[1 1 1] Mouse over
  (bind _actorclicked (`/Game/Blueprints/BP_IntelligentViewPawn.isActorClicked` (`/Game/Blueprints/All/StaticLib.GetPawn`) self))
  (if (not _actorclicked)
    (`self.EnableOutline`)))

(event `self.Cylinder.OnEndCursorOver`
  (params (TouchedComponent :type "PrimitiveComponent Object Reference"))
  ;[1 1 1] Mouse over
  (bind _actorclicked (`/Game/Blueprints/BP_IntelligentViewPawn.isActorClicked` (`/Game/Blueprints/All/StaticLib.GetPawn`) self))
  (if (not _actorclicked)
    (`self.DisableOutline`)))

(event `self.Cylinder.OnClicked`
  (params (TouchedComponent :type "PrimitiveComponent Object Reference") (ButtonPressed :type "Key Structure"))
  ;[1 1 1] Mouse click
  (`/Game/Blueprints/BP_IntelligentViewPawn.SetCurrentClickActor` (`/Game/Blueprints/All/StaticLib.GetPawn`) self)
  (`self.ToggleGoal` true))

(event `ActionCenter`
  (bind _currentthreat (`self.currentThreat`))
  (switch `/Game/Blueprints/All/EPatrolState` (`self.patrolState`)
    (:`NewEnumerator3`
      ;[1 1 1] Random moving
      (`self.PickRandomGoal` :!label _label)
      (set `self.patrolState` "NewEnumerator1")
      (`|AIMoveTo` self (`self.currentGoal`) null
        (:`then`
          (`/Engine/EditorBlueprintResources/StandardMacros.IsValid` (`self.goalRepresentationRef`)
            (:`Is Valid`
              (`self.ToggleGoal` true))))
        (:`OnSuccess`
          (set `self.patrolState` "NewEnumerator4" :!label _label_2)
          (`self.ActionCenter`))
        (:`OnFail`
          (goto _label_2))))
    (:`NewEnumerator4`
      (goto _label))
    (:`NewEnumerator7`
      ;[1 1 1] Moving to threat
      (`|AIMoveTo` self (0.0 0.0 0.0) _currentthreat
        (:`then`
          (set `self.currentGoal` (`self.K2_GetActorLocation` _currentthreat))
          (`self.ToggleGoal` true))
        (:`OnSuccess`
          (set `self.patrolState` "NewEnumerator8" :!label _label_3)
          (`self.ActionCenter`))
        (:`OnFail`
          (goto _label_3))))
    (:`NewEnumerator8`
      ;[1 1 1] threat handling
      (`KismetSystemLibrary.Delay` (`KismetMathLibrary.RandomFloatInRange` 1.0 8.0))
      (`self.K2_DestroyActor` (`self.currentThreat`))
      (`self.FinishOrder`)
      (set `self.currentThreat` null)
      (`/Game/Blueprints/BP_FunctionLibrary.UpdateSelectedWidget`)
      (set `self.patrolState` "NewEnumerator9")
      (`self.ActionCenter`))
    (:`NewEnumerator9`
      ;[1 1 1] Check new order
      (bind _outactors (`GameplayStatics.GetAllActorsOfClass` "/Game/Blueprints/Model/BP_HeadQuarter.BP_HeadQuarter_C"))
      (bind _ordersend (`/Game/Blueprints/Model/BP_HeadQuarter.NotifyPatrolOnCrime` (`|GetArrayItem` _outactors) self))
      (if (not _ordersend)
        (set `self.patrolState` "NewEnumerator4")
        (`self.ActionCenter`)))))

(fn `InitSetup`
  (bind _returnvalue (`KismetMaterialLibrary.CreateDynamicMaterialInstance` "/Game/Materials/M_Patrol.M_Patrol"))
  (bind _output_get (set `self.dynamicMaterial` _returnvalue))
  (`PrimitiveComponent.SetMaterial` (`self.Cylinder`) 0 _output_get)
  (bind _returnvalue_2 (`|SpawnActorFromClass` "/Game/Blueprints/Model/BP_Navi.BP_Navi_C" (`self.GetTransform`) "Undefined" "OverrideRootScale" self null))
  (`self.K2_AttachToComponent` _returnvalue_2 (`self.CapsuleComponent`) "None" "SnapToTarget" "SnapToTarget" "SnapToTarget" true)
  (`self.AssignNavigation` _returnvalue_2)
  (for _ (range 1 (+ (`self.officersInPatrol`) 1))
    (bind _returnvalue_3 (`|SpawnActorFromClass` "/Game/Blueprints/Model/BP_Policeman.BP_Policeman_C" (`self.GetTransform`) "Undefined" "OverrideRootScale" self null))
    (`self.K2_AttachToComponent` _returnvalue_3 (`self.CapsuleComponent`) "None" "SnapToTarget" "SnapToTarget" "SnapToTarget" true)
    (`self.AddPolicemanToPatrol` _returnvalue_3)))

(fn `PickRandomGoal`
  (set `self.currentGoal` (`/Game/Blueprints/All/StaticLib.GetRandomPointOnRoad`))
  (return))

(fn `ToggleGoal`
  (params (show :type Boolean))
  (bind _goalrepresentationref (`self.goalRepresentationRef`))
  (bind _goalrepresentationref_2 (`self.goalRepresentationRef`))
  (if show
    (`/Engine/EditorBlueprintResources/StandardMacros.IsValid` _goalrepresentationref
      (:`Is Valid`
        (`self.K2_DestroyActor` _goalrepresentationref))
      (:`Is Not Valid`
        _))
    (bind _returnvalue (`|SpawnActorFromClass` "/Game/Blueprints/Threats/BP_GoalRepresentation.BP_GoalRepresentation_C" (`KismetMathLibrary.MakeTransform` (`self.currentGoal`)) "Undefined" "OverrideRootScale" null null))
    (set `self.goalRepresentationRef` _returnvalue)
    (else
      (`/Engine/EditorBlueprintResources/StandardMacros.IsValid` _goalrepresentationref_2
        (:`Is Valid`
          (`self.K2_DestroyActor` _goalrepresentationref_2))))))

(fn `UserConstructionScript`)