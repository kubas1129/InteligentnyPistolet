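; BP_Policeman is a policeman Blueprint that equips itself with a pistol and a smartwatch when play begins.
; BeginPlay calls InitSetup, which spawns BP_Pistol and BP_SmartWatch at the policeman's transform with itself as owner.
; Each is attached to DefaultSceneRoot with keep-relative rules, then handed to AssignPistol or AssignSmartWatch.
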(event `self.ReceiveBeginPlay`
  (`self.InitSetup`))

(fn `InitSetup`
  (bind _returnvalue (`|SpawnActorFromClass` "/Game/Blueprints/Model/BP_Pistol.BP_Pistol_C" (`self.GetTransform`) "Undefined" "OverrideRootScale" self null))
  (`self.K2_AttachToComponent` _returnvalue (`self.DefaultSceneRoot`) "None" "KeepRelative" "KeepRelative" "KeepRelative" true)
  (`self.AssignPistol` _returnvalue)
  (bind _returnvalue_2 (`|SpawnActorFromClass` "/Game/Blueprints/Model/BP_SmartWatch.BP_SmartWatch_C" (`self.GetTransform`) "Undefined" "OverrideRootScale" self null))
  (`self.K2_AttachToComponent` _returnvalue_2 (`self.DefaultSceneRoot`) "None" "KeepRelative" "KeepRelative" "KeepRelative" true)
  (`self.AssignSmartWatch` _returnvalue_2))

(fn `UserConstructionScript`)