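; BP_HeadQuarter is a selectable headquarters actor that spawns and registers its patrols when play begins.
; SpawnPatrols loops with a two-second delay, spawning the configured number of BP_Patrol actors at SpawnPoint, each with a random officer count.
; Hovering the Cube toggles a custom-depth outline unless the pawn reports this actor as clicked.
; Clicking the Cube sets it as the pawn's current clicked actor.
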(event `self.ReceiveBeginPlay`
  (`|ExecutionSequence`
    (:`then_0`
      (`self.SpawnPatrols`))))

(event `/Game/Blueprints/All/BP_OutlineInterface.EnableOutline`
  ;[1 1 1] Outline interface
  (`PrimitiveComponent.SetRenderCustomDepth` (`self.Cube`) true))

(event `/Game/Blueprints/All/BP_OutlineInterface.DisableOutline`
  ;[1 1 1] Outline interface
  (`PrimitiveComponent.SetRenderCustomDepth` (`self.Cube`) false))

(event `self.Cube.OnBeginCursorOver`
  (params (TouchedComponent :type "PrimitiveComponent Object Reference"))
  ;[1 1 1] Mouse over
  (bind _actorclicked (`/Game/Blueprints/BP_IntelligentViewPawn.isActorClicked` (`/Game/Blueprints/All/StaticLib.GetPawn`) self))
  (if (not _actorclicked)
    (`/Game/Blueprints/All/BP_OutlineInterface.EnableOutline`)))

(event `self.Cube.OnEndCursorOver`
  (params (TouchedComponent :type "PrimitiveComponent Object Reference"))
  ;[1 1 1] Mouse over
  (bind _actorclicked (`/Game/Blueprints/BP_IntelligentViewPawn.isActorClicked` (`/Game/Blueprints/All/StaticLib.GetPawn`) self))
  (if (not _actorclicked)
    (`/Game/Blueprints/All/BP_OutlineInterface.DisableOutline`)))

(event `self.Cube.OnClicked`
  (params (TouchedComponent :type "PrimitiveComponent Object Reference") (ButtonPressed :type "Key Structure"))
  ;[1 1 1] Mouse click
  (`/Game/Blueprints/BP_IntelligentViewPawn.SetCurrentClickActor` (`/Game/Blueprints/All/StaticLib.GetPawn`) self))

(fn `UserConstructionScript`)